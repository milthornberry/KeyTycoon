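; BP_Knife is an interactable knife tool that cuts or skins fruit in front of the first-person character.
; Both Interact and AltInteract sphere-trace from the player camera and act only on actors tagged "Fruit", with debug drawing and prints left on.
; Interact hides and destroys the fruit, spawning BP_CutFruit at its transform.
; AltInteract fakes skinning by swapping the material on the fruit's primitive components.
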(event `self.ReceiveBeginPlay`
  (bind _returnvalue (`GameplayStatics.GetActorOfClass` "/Game/FirstPerson/Blueprints/BP_FirstPersonCharacter.BP_FirstPersonCharacter_C"))
  (set `self.FPCharacter` _returnvalue))

(event `/Game/BPI_PickupItem.Interact`
  (bind _firstpersoncamera (`/Game/FirstPerson/Blueprints/BP_FirstPersonCharacter.FirstPersonCamera` (`self.FPCharacter`)))
  (bind _returnvalue (`SceneComponent.K2_GetComponentLocation` _firstpersoncamera))
  ; Cut the apple
  (`KismetSystemLibrary.PrintString` "Cutting apple")
  (bind _outhit (`KismetSystemLibrary.SphereTraceSingle` :`Start` _returnvalue :`End` (+ _returnvalue (* (`SceneComponent.GetForwardVector` _firstpersoncamera) 200.0)) :`Radius` 20.0 :`TraceChannel` "TraceTypeQuery1" :`DrawDebugType` "ForDuration"))
  (bind (_bblockinghit _binitialoverlap _time _distance _location _impactpoint _normal _impactnormal _physmat _hitactor) (`GameplayStatics.BreakHitResult` _outhit))
  (`KismetSystemLibrary.PrintString` (`KismetStringLibrary.Concat_StrStr` "found" (`KismetSystemLibrary.GetDisplayName` _hitactor)))
  (if (`self.ActorHasTag` _hitactor "Fruit")
    (bind _output_get (set `self.FoundFruit` _hitactor))
    (`self.SetActorHiddenInGame` _output_get true)
    (`|SpawnActorFromClass` "/Game/BP_CutFruit.BP_CutFruit_C" (`self.GetTransform` _output_get) "Undefined" "MultiplyWithRoot" null null)
    (`self.K2_DestroyActor` _output_get)))

(event `/Game/BPI_PickupItem.AltInteract`
  (bind _firstpersoncamera (`/Game/FirstPerson/Blueprints/BP_FirstPersonCharacter.FirstPersonCamera` (`self.FPCharacter`)))
  (bind _returnvalue (`SceneComponent.K2_GetComponentLocation` _firstpersoncamera))
  ; Skin the apple
  (`KismetSystemLibrary.PrintString` "Skinning apple")
  (bind _outhit (`KismetSystemLibrary.SphereTraceSingle` :`Start` _returnvalue :`End` (+ _returnvalue (* (`SceneComponent.GetForwardVector` _firstpersoncamera) 200.0)) :`Radius` 20.0 :`TraceChannel` "TraceTypeQuery1" :`DrawDebugType` "ForDuration"))
  (bind (_bblockinghit _binitialoverlap _time _distance _location _impactpoint _normal _impactnormal _physmat _hitactor) (`GameplayStatics.BreakHitResult` _outhit))
  (`KismetSystemLibrary.PrintString` (`KismetStringLibrary.Concat_StrStr` "found" (`KismetSystemLibrary.GetDisplayName` _hitactor)))
  (if (`self.ActorHasTag` _hitactor "Fruit")
    (bind _output_get (set `self.FoundFruit` _hitactor))
    (`PrimitiveComponent.SetMaterial` (`self.K2_GetComponentsByClass` _output_get "/Script/Engine.PrimitiveComponent") 0 "/Game/Materials/DonutBase1.DonutBase1")))

(fn `UserConstructionScript`)