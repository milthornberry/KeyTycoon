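; BP_Chest is an interactable chest actor that opens with a menu and animated hinge.
; BeginPlay pre-creates the WBP_ChestMenu widget and caches the first-person character.
; OpenChest shows the menu, disables player movement, switches to UI-only input with a cursor, and plays a timeline rotating the hinge.
; CloseChest only animates the hinge back through a second timeline, without restoring movement, input or removing the menu.
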(event `self.ReceiveBeginPlay`
  (bind _returnvalue (`|CreateWidget` "/Game/WBP_ChestMenu.WBP_ChestMenu_C" (`GameplayStatics.GetPlayerController` 0)))
  (set `self.ChestMenuWidget` _returnvalue)
  (bind _returnvalue_2 (`GameplayStatics.GetActorOfClass` "/Game/FirstPerson/Blueprints/BP_FirstPersonCharacter.BP_FirstPersonCharacter_C"))
  (set `self.FirstPerson` _returnvalue_2))

(event `OpenChest`
  (bind _returnvalue (`GameplayStatics.GetPlayerController` 0))
  (`UserWidget.AddToViewport` (`self.ChestMenuWidget`) 0)
  (`CharacterMovementComponent.DisableMovement` (`Character.CharacterMovement` (`self.FirstPerson`)))
  (set `PlayerController.bShowMouseCursor` true _returnvalue)
  (`WidgetBlueprintLibrary.SetInputMode_UIOnlyEx` _returnvalue (`self.ChestMenuWidget`))
  (bind (_direction _chestopen) (`Timeline|ChestOpen`)
    (:`Update`
      (`SceneComponent.K2_SetRelativeRotation` (`self.Hinge`) (`KismetMathLibrary.RLerp` (struct :`Pitch` -90.0 :`Yaw` 90.0 :`Roll` -90.0) (`KismetMathLibrary.MakeRotator` -90.0 -40.0 90.0) _chestopen true) false false))))

(event `CloseChest`
  (bind (_direction _chestopen) (`Timeline|Timeline` :!via `PlayFromStart`)
    (:`Update`
      (`SceneComponent.K2_SetRelativeRotation` (`self.Hinge`) (`KismetMathLibrary.RLerp` (struct :`Pitch` -40.0 :`Yaw` 90.0 :`Roll` -90.0) (`KismetMathLibrary.MakeRotator` -90.0 -90.0 90.0) _chestopen true) false false))))

(fn `UserConstructionScript`)