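; BP_KeyMaterial is a collectible actor that the first-person player picks up by overlapping it.
; On overlap it increments the character's MaterialCount, prints the new total and destroys itself.
; When the count reaches five, it updates the character's dialogue widget to show that the materials have been gathered.
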(event `self.Collision.OnComponentBeginOverlap`
  (params (OverlappedComponent :type "PrimitiveComponent Object Reference") (OtherActor :type "Actor Object Reference") (OtherComp :type "PrimitiveComponent Object Reference") (OtherBodyIndex :type Integer) (bFromSweep :type Boolean) (SweepResult :type "HitResult Structure (by ref)"))
  ; When material is overlapped, add to the material count and display the new value in a print string. Then destroy the material actor.
  (bind _asbp_first_person_character (cast `/Game/FirstPerson/Blueprints/BP_FirstPersonCharacter` OtherActor))
  (bind _materialcount (`/Game/FirstPerson/Blueprints/BP_FirstPersonCharacter.MaterialCount` _asbp_first_person_character))
  (`/Engine/EditorBlueprintResources/StandardMacros.IncrementInt` _materialcount
    (:`  `
      (`KismetSystemLibrary.PrintString` (`KismetStringLibrary.Concat_StrStr` (`self.SmaterialCount`) (`KismetStringLibrary.Conv_IntToString` _materialcount)))
      (if (== _materialcount 5)
        (`/Game/WBP_Dialogue.SetHasMaterialsText` (`/Game/FirstPerson/Blueprints/BP_FirstPersonCharacter.DialogueWidget` _asbp_first_person_character)))
      (`self.K2_DestroyActor`))))

(fn `UserConstructionScript`)