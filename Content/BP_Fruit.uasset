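; BP_Fruit is a held-item fruit actor that can be eaten or thrown by the first-person character.
; Interact prints an eating message and destroys the actor.
; AltInteract, labeled as adding to a recipe, detaches the fruit and launches its physics-enabled Sphere along the camera's forward vector with a velocity-change impulse.
; After a delay it stops the physics and resets the held item on the character cached at BeginPlay.
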(event `self.ReceiveBeginPlay`
  (bind _returnvalue (`GameplayStatics.GetActorOfClass` "/Game/FirstPerson/Blueprints/BP_FirstPersonCharacter.BP_FirstPersonCharacter_C"))
  (set `self.FPCharacter` _returnvalue))

(event `/Game/BPI_Item.Interact`
  (`KismetSystemLibrary.PrintString` "Eating fruit")
  (`self.K2_DestroyActor`))

(event `/Game/BPI_Item.AltInteract`
  (`KismetSystemLibrary.PrintString` "Adding fruit to recipe")
  (`self.SetActorEnableCollision` true)
  (`self.K2_DetachFromActor` self "KeepWorld" "KeepRelative" "KeepRelative")
  (`PrimitiveComponent.SetSimulatePhysics` (`self.Sphere`) true)
  (`PrimitiveComponent.AddImpulse` (`self.Sphere`) (* (`SceneComponent.GetForwardVector` (`/Game/FirstPerson/Blueprints/BP_FirstPersonCharacter.FirstPersonCamera` (`self.FPCharacter`))) (500.0 500.0 500.0)) "None" true)
  (`KismetSystemLibrary.Delay` 2.0)
  (`PrimitiveComponent.SetSimulatePhysics` (`self.Sphere`) false)
  (`/Game/FirstPerson/Blueprints/BP_FirstPersonCharacter.ResetHeldItem` (`self.FPCharacter`)))

(fn `UserConstructionScript`)