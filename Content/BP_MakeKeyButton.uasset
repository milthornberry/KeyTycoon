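; BP_MakeKeyButton is a button actor that makes a key in exchange for the player's materials.
; Its Interact event deducts a fixed material cost from the cached first-person character, prints the new total, and spawns a physics-simulated BP_Key at a hardcoded location.
; Box overlaps track whether the player is near, but Interact checks neither that flag nor the material balance.
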(event `self.ReceiveBeginPlay`
  (bind _returnvalue (`GameplayStatics.GetActorOfClass` "/Game/FirstPerson/Blueprints/BP_FirstPersonCharacter.BP_FirstPersonCharacter_C"))
  (set `self.FPCharacter` _returnvalue))

(event `/Game/BPI_PickupItem.Interact`
  (bind _fpcharacter (`self.FPCharacter`))
  (bind _output_get (set `/Game/FirstPerson/Blueprints/BP_FirstPersonCharacter.MaterialCount` (- (`/Game/FirstPerson/Blueprints/BP_FirstPersonCharacter.MaterialCount` _fpcharacter) 5) _fpcharacter))
  (`KismetSystemLibrary.PrintString` (`KismetStringLibrary.Conv_IntToString` _output_get) true true (struct :`G` 0.66 :`B` 1.0 :`A` 1.0) 30.0 "Total Count")
  (bind _returnvalue (`|SpawnActorFromClass` "/Game/BP_Key.BP_Key_C" (`KismetMathLibrary.MakeTransform` (-78.876824 -534.647486 117.309219)) "Undefined" "MultiplyWithRoot" null null))
  (`PrimitiveComponent.SetSimulatePhysics` (`/Game/BP_Key.Cube` _returnvalue) true))

(event `self.Box.OnComponentBeginOverlap`
  (params (OverlappedComponent :type "PrimitiveComponent Object Reference") (OtherActor :type "Actor Object Reference") (OtherComp :type "PrimitiveComponent Object Reference") (OtherBodyIndex :type Integer) (bFromSweep :type Boolean) (SweepResult :type "HitResult Structure (by ref)"))
  (cast `/Game/FirstPerson/Blueprints/BP_FirstPersonCharacter` OtherActor)
  (set `self.BNearButton` true))

(event `self.Box.OnComponentEndOverlap`
  (params (OverlappedComponent :type "PrimitiveComponent Object Reference") (OtherActor :type "Actor Object Reference") (OtherComp :type "PrimitiveComponent Object Reference") (OtherBodyIndex :type Integer))
  (cast `/Game/FirstPerson/Blueprints/BP_FirstPersonCharacter` OtherActor)
  (set `self.BNearButton` false))

(fn `UserConstructionScript`)